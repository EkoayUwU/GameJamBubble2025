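; BP_Trap is a trap that respawns the player character if it is still inside the collider when the trap snaps shut.
; Overlap opens a gate and starts the FenetreMort delay; leaving closes the gate, so escaping in time avoids respawn.
; After the delay, it zeroes velocity and calls RespawnEvent if the gate is open, then plays close and, later, reopen animations.
; A DoOnce blocks retriggering until the cycle finishes.
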(event OnComponentBeginOverlap(Collider)
  (params (OverlappedComponent :type Primitive%20Component%20Object%20Reference) (OtherActor :type Actor%20Object%20Reference) (OtherComp :type Primitive%20Component%20Object%20Reference) (OtherBodyIndex :type Integer) (bFromSweep :type Boolean) (SweepResult :type Hit%20Result%20Structure%20%28by%20ref%29))
  (bind _asbp_third_person_character (Utilities|Casting|CastToBP_ThirdPersonCharacter OtherActor))
  (Utilities|FlowControl|Sequence
    (:then_0
      (Utilities|FlowControl|DelayUntilNextTick)
      (Utilities|FlowControl|DoOnce false :!label _label
        (:Completed
          (Utilities|FlowControl|Delay (Variables|Parameters|GetFenetre%20Mort))
          (Utilities|FlowControl|Sequence
            (:then_0
              (Utilities|FlowControl|Gate true :!label _label_2
                (:Exit
                  (Variables|/Script/Engine.MovementComponent|SetVelocity (Variables|/Script/Engine.Character|GetCharacterMovement _asbp_third_person_character) "0, 0, 0")
                  (Default|RespawnEvent _asbp_third_person_character))))
            (:then_1
              (Components|Animation|PlayAnimation (Variables|Default|GetSM_Trap) "/Game/GameBank/Core/Animation/AS_Trap_Close.AS_Trap_Close" false)
              (Utilities|FlowControl|Delay (Variables|Parameters|GetDelay%20avant%20Reouverture))
              (Components|Animation|PlayAnimation (Variables|Default|GetSM_Trap) "/Game/GameBank/Core/Animation/AS_Trap_Open.AS_Trap_Open" false)
              (Utilities|FlowControl|Delay 0.2)
              (goto _label Reset))))))
    (:then_1
      (goto _label_2 Open))))

(event OnComponentEndOverlap(Collider)
  (params (OverlappedComponent :type Primitive%20Component%20Object%20Reference) (OtherActor :type Actor%20Object%20Reference) (OtherComp :type Primitive%20Component%20Object%20Reference) (OtherBodyIndex :type Integer))
  (Utilities|Casting|CastToBP_ThirdPersonCharacter OtherActor)
  (Utilities|FlowControl|Gate true) ; enters at Close
)

(event EventBeginPlay
  (Components|Animation|PlayAnimation (Variables|Default|GetSM_Trap) "/Game/GameBank/Core/Animation/AS_Trap_Idle.AS_Trap_Idle" true))

(fn ConstructionScript)