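; BP_Collectibles is a coin-style pickup that the player collects by touching it.
; After a short delay a timeline bobs the mesh up and down, while Tick spins it at a fixed per-frame rate.
; On overlap with BP_ThirdPersonCharacter it passes its CoinValue and OtherValue to the character's ChangeCoinUi, then destroys itself.
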(event OnComponentBeginOverlap(SM_Collectible)
  (params (OverlappedComponent :type Primitive%20Component%20Object%20Reference) (OtherActor :type Actor%20Object%20Reference) (OtherComp :type Primitive%20Component%20Object%20Reference) (OtherBodyIndex :type Integer) (bFromSweep :type Boolean) (SweepResult :type Hit%20Result%20Structure%20%28by%20ref%29))
  (bind _asbp_third_person_character (Utilities|Casting|CastToBP_ThirdPersonCharacter OtherActor))
  (Default|ChangeCoinUi _asbp_third_person_character (Variables|Parameters|GetCoin%20Value) (Variables|Parameters|GetOther%20Value))
  (Actor|DestroyActor))

(event EventBeginPlay
  (bind _sm_collectible (Variables|Default|GetSM_Collectible))
  (bind _relativelocation (Variables|/Script/Engine.SceneComponent|GetRelativeLocation _sm_collectible))
  (Utilities|FlowControl|Delay 0.2)
  (Components|Timeline|SetPlayRate (Variables|Default|GetUpDown) 2.0)
  (bind _alpha (Timeline|UpDown PlayFromStart)
    (:Update
      (Transformation|SetRelativeLocation _sm_collectible (Math|Vector|MakeVector (.x _relativelocation) (.y _relativelocation) (Math|Float|Lerp 5e+01 65.0 _alpha)) false false))))

(event EventTick
  (params (DeltaSeconds :type Float%20%28single-precision%29))
  (Transformation|AddRelativeRotation (Variables|Default|GetSM_Collectible) "0.000000,0.200000,0.000000" false false))

(fn ConstructionScript)