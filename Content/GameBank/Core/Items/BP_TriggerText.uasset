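; BP_TriggerText is a trigger actor that toggles an on-screen text message as the player passes through it.
; On BeginPlay it creates a WBP_TextInfo widget, adds it to the viewport and fills it with the Text variable.
; EnterBox and ExitBox overlaps by BP_ThirdPersonCharacter each call the widget's Toggle, with a separate DoOnce limiting each box to a single firing.
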(event OnComponentBeginOverlap(EnterBox)
  (params (OverlappedComponent :type Primitive%20Component%20Object%20Reference) (OtherActor :type Actor%20Object%20Reference) (OtherComp :type Primitive%20Component%20Object%20Reference) (OtherBodyIndex :type Integer) (bFromSweep :type Boolean) (SweepResult :type Hit%20Result%20Structure%20%28by%20ref%29))
  (Utilities|Casting|CastToBP_ThirdPersonCharacter OtherActor)
  (Utilities|FlowControl|DoOnce false
    (:Completed
      (Default|Toggle (stale EventBeginPlay _returnvalue)))))

(event OnComponentBeginOverlap(ExitBox)
  (params (OverlappedComponent :type Primitive%20Component%20Object%20Reference) (OtherActor :type Actor%20Object%20Reference) (OtherComp :type Primitive%20Component%20Object%20Reference) (OtherBodyIndex :type Integer) (bFromSweep :type Boolean) (SweepResult :type Hit%20Result%20Structure%20%28by%20ref%29))
  (Utilities|Casting|CastToBP_ThirdPersonCharacter OtherActor)
  (Utilities|FlowControl|DoOnce false
    (:Completed
      (Default|Toggle (stale EventBeginPlay _returnvalue)))))

(event EventBeginPlay
  (bind _returnvalue (UserInterface|CreateWidget "/Game/GameBank/Core/UI/WBP_TextInfo.WBP_TextInfo_C"))
  (UserInterface|Viewport|AddtoViewport _returnvalue 0)
  (Default|SetText _returnvalue (Variables|Parameters|GetText)))

(fn ConstructionScript)