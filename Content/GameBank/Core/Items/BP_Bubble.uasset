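; Player-fired bubble projectile that stops on contact with other actors (except collectibles) and becomes a bouncy jump bumper.
; It grows while attached, detaches toward the camera trace hit, then travels on a looping timer, expiring if nothing stops it.
; A sphere trace flags wall landings, which launch the player straight up; others scale horizontal velocity by player state.
; Tuning comes from the player's DAPP, and KillBuble plays a dissolve before destruction.
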(event OnComponentBeginOverlap(MSH_Bubble)
  (params (OverlappedComponent :type Primitive%20Component%20Object%20Reference) (OtherActor :type Actor%20Object%20Reference) (OtherComp :type Primitive%20Component%20Object%20Reference) (OtherBodyIndex :type Integer) (bFromSweep :type Boolean) (SweepResult :type Hit%20Result%20Structure%20%28by%20ref%29))
  (bind _returnvalue (Transformation|GetActorLocation))
  (bind _playerref (Variables|Parameters|GetPlayerRef))
  (bind _playerref_2 (Variables|Parameters|GetPlayerRef))
  (bind _da_pp (Variables|/Game/GameBank/Core/Characters/ThirdPerson/Blueprints/BP_ThirdPersonCharacter.BP_ThirdPersonCharacter_C|GetDA_PP _playerref))
  (bind _currentplayerstate (Variables|/Game/GameBank/Core/Characters/ThirdPerson/Blueprints/BP_ThirdPersonCharacter.BP_ThirdPersonCharacter_C|GetCurrentPlayerState _playerref_2))
  (bind _returnvalue_2 (Utilities|Enum|Equal(Enum) _currentplayerstate "NewEnumerator3"))
  (bind _bumper_defaultforce (Variables|/Game/GameBank/Core/Data/BP_DA_PP.BP_DA_PP_C|GetBumper_DefaultForce _da_pp))
  (bind _bumper_dashforce (Variables|/Game/GameBank/Core/Data/BP_DA_PP.BP_DA_PP_C|GetBumper_DashForce _da_pp))
  (bind _returnvalue_3 (Math|Float|SelectFloat _bumper_dashforce _bumper_defaultforce _returnvalue_2))
  ;[1 1 1] Check Wall hit Bubble
  (if (Variables|Parameters|GetbStopTravel)
    (if (== OtherActor (Variables|Parameters|GetPlayerRef))
      (Utilities|FlowControl|DoOnce false :!label _label
        (:Completed
          (Utilities|FlowControl|Sequence
            (:then_0
              ;[1 1 1] JumpOnBubble
              (if (Variables|Parameters|GetbIsWalled)
                (Variables|/Script/Engine.MovementComponent|SetVelocity (Variables|/Script/Engine.Character|GetCharacterMovement (Variables|Parameters|GetPlayerRef)) "0, 0, 0")
                (Character|LaunchCharacter (Variables|Parameters|GetPlayerRef) (Math|Vector|MakeVector 0.0 0.0 (Variables|/Game/GameBank/Core/Data/BP_DA_PP.BP_DA_PP_C|GetBumper_UpwardForce (Variables|/Game/GameBank/Core/Characters/ThirdPerson/Blueprints/BP_ThirdPersonCharacter.BP_ThirdPersonCharacter_C|GetDA_PP (Variables|Parameters|GetPlayerRef)))) true true)
                (else
                  (Character|LaunchCharacter (Variables|Parameters|GetPlayerRef) (Math|Vector|MakeVector (* (.x (Variables|/Script/Engine.MovementComponent|GetVelocity (Variables|/Script/Engine.Character|GetCharacterMovement (Variables|Parameters|GetPlayerRef)))) _returnvalue_3) (* (.y (Variables|/Script/Engine.MovementComponent|GetVelocity (Variables|/Script/Engine.Character|GetCharacterMovement (Variables|Parameters|GetPlayerRef)))) _returnvalue_3) 1e+03) false true))))
            (:then_1
              (Utilities|FlowControl|Delay 0.35)
              (goto _label Reset))))))
    (elif (Math|Boolean|ANDBoolean (!= OtherActor self) (!= OtherActor (Variables|Parameters|GetPlayerRef)) (!= (Utilities|GetClass OtherActor) "/Game/GameBank/Core/Items/BP_Collectibles.BP_Collectibles_C"))
      (Utilities|FlowControl|DoOnce false
        (:Completed
          (Utilities|FlowControl|Delay 0.01)
          (Variables|Parameters|SetbStopTravel true)
          (bind (_outhit _returnvalue_4) (Collision|SphereTraceByChannel _returnvalue _returnvalue 65.0 "TraceTypeQuery1" false (Utilities|Array|MakeArray self (Variables|Parameters|GetPlayerRef)) "None"))
          (if (and _returnvalue_4 (Math|Float|NearlyEqual(Float) (Math|Vector|DotProduct (.Normal (Collision|BreakHitResult _outhit)) (Math|Vector|VectorUp)) 0.0 0.0))
            (Variables|Parameters|SetbIsWalled true)
            (else
              (Variables|Parameters|SetbIsWalled false))))))))

(event Custom|Bubble_Travel
  ;[1 1 1] Init + Bubble Travel
  (if (not (Variables|Parameters|GetbStopTravel))
    (Transformation|SetActorLocation self (+ (Transformation|GetActorLocation) (* (Transformation|GetActorForwardVector) (Variables|/Game/GameBank/Core/Data/BP_DA_PP.BP_DA_PP_C|GetBubbleSpeed (Variables|/Game/GameBank/Core/Characters/ThirdPerson/Blueprints/BP_ThirdPersonCharacter.BP_ThirdPersonCharacter_C|GetDA_PP (Variables|Parameters|GetPlayerRef))))) false false)
    (Math|Integer|IncrementInt (Variables|Default|Getint)
      (:%20%20
        (if (Variables|Parameters|GetbStopTravel)
          (Utilities|Time|ClearandInvalidateTimerbyHandle (Variables|Default|GetTimerHandle)))))))

(event Custom|KillBuble
  (bind _playerref (Variables|Parameters|GetPlayerRef))
  (bind _da_pp (Variables|/Game/GameBank/Core/Characters/ThirdPerson/Blueprints/BP_ThirdPersonCharacter.BP_ThirdPersonCharacter_C|GetDA_PP _playerref))
  (bind _bubblemaxscale (Variables|/Game/GameBank/Core/Data/BP_DA_PP.BP_DA_PP_C|GetBubbleMaxScale _da_pp))
  (Collision|SetActorEnableCollision false)
  (bind _alpha (Timeline|LerpDissolve PlayFromStart)
    (:Update
      (Rendering|Material|SetScalarParameterValue (Variables|Default|GetDynMat) "Dissolve" (Math|Float|Lerp 0.0 4.0 _alpha) :!class /Script/Engine.MaterialInstanceDynamic)
      (Transformation|SetWorldScale3D (Variables|Default|GetMSH_Bubble) (Math|Conversions|ToVector(Float) (Math|Float|Lerp _bubblemaxscale (+ _bubblemaxscale 0.5) _alpha))))
    (:Finished
      (Actor|DestroyActor))))

(event EventBeginPlay
  (bind _msh_bubble (Variables|Default|GetMSH_Bubble))
  ;[1 1 1] Init + Bubble Travel
  (bind _returnvalue (Rendering|Material|CreateDynamicMaterialInstance _msh_bubble 0 (Rendering|Material|GetMaterial _msh_bubble 0) "None" :!class /Script/Engine.PrimitiveComponent))
  (Variables|Default|SetDynMat _returnvalue)
  (bind _asbp_third_person_character (Utilities|Casting|CastToBP_ThirdPersonCharacter (Variables|Actor|GetInstigator)))
  (Variables|Parameters|SetPlayerRef _asbp_third_person_character)
  (Components|Timeline|SetPlayRate (Variables|Default|GetLerp%20Grow%20Bubble) (Variables|/Game/GameBank/Core/Data/BP_DA_PP.BP_DA_PP_C|GetBubbleGrowSpeed (Variables|/Game/GameBank/Core/Characters/ThirdPerson/Blueprints/BP_ThirdPersonCharacter.BP_ThirdPersonCharacter_C|GetDA_PP (Variables|Parameters|GetPlayerRef))))
  (bind _alpha (Timeline|Lerp%20Grow%20Bubble PlayFromStart)
    (:Update
      (Transformation|SetRelativeScale3D (Variables|Default|GetMSH_Bubble) (Math|Conversions|ToVector(Float) (Math|Float|Lerp 0.05 (Variables|/Game/GameBank/Core/Data/BP_DA_PP.BP_DA_PP_C|GetBubbleMaxScale (Variables|/Game/GameBank/Core/Characters/ThirdPerson/Blueprints/BP_ThirdPersonCharacter.BP_ThirdPersonCharacter_C|GetDA_PP (Variables|Parameters|GetPlayerRef))) _alpha))))
    (:Finished
      (bind (_outhit _returnvalue_2) (Collision|LineTraceByChannel (+ (Transformation|GetWorldLocation (Variables|/Game/GameBank/Core/Characters/ThirdPerson/Blueprints/BP_ThirdPersonCharacter.BP_ThirdPersonCharacter_C|GetFollowCamera (Variables|Parameters|GetPlayerRef))) (* (Math|Vector|GetForwardVector (Variables|/Game/GameBank/Core/Characters/ThirdPerson/Blueprints/BP_ThirdPersonCharacter.BP_ThirdPersonCharacter_C|GetFollowCamera (Variables|Parameters|GetPlayerRef))) 25.0)) (+ (* (Math|Vector|GetForwardVector (Variables|/Game/GameBank/Core/Characters/ThirdPerson/Blueprints/BP_ThirdPersonCharacter.BP_ThirdPersonCharacter_C|GetFollowCamera (Variables|Parameters|GetPlayerRef))) 1e+04) (Transformation|GetWorldLocation (Variables|/Game/GameBank/Core/Characters/ThirdPerson/Blueprints/BP_ThirdPersonCharacter.BP_ThirdPersonCharacter_C|GetFollowCamera (Variables|Parameters|GetPlayerRef)))) "TraceTypeQuery1" false 0 "None"))
      (if _returnvalue_2
        (Transformation|SetActorRotation self (Math|Rotator|FindLookatRotation (Transformation|GetActorLocation) (.ImpactPoint (Collision|BreakHitResult _outhit)))))
      (Transformation|DetachFromActor "KeepWorld" "KeepWorld" "KeepWorld")
      (bind _returnvalue_3 (Utilities|Time|SetTimerbyEvent (delegate Custom|Bubble_Travel) 0.01 true))
      (Variables|Default|SetTimerHandle _returnvalue_3)
      (Utilities|FlowControl|Delay 7.5)
      (if (not (Variables|Parameters|GetbStopTravel))
        (Actor|DestroyActor)))))

(fn ConstructionScript)